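; Key_BP is a key actor that highlights itself and shows an interact prompt when approached.
; BeginPlay caches the StaticMesh's original material, which overlap begin swaps for a Glow material and overlap end restores.
; Any overlapping actor triggers the swap, while only a BP_FirstPersonCharacter gets its EToInteract prompt shown and hidden.
; The Blueprint itself contains no input or pickup logic.
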(event `self.ReceiveBeginPlay`
  (set `self.originalMaterial` (`PrimitiveComponent.GetMaterial` (`self.StaticMesh`) 0)))

(event `self.ReceiveActorBeginOverlap`
  (params (OtherActor :type "Actor Object Reference"))
  (`PrimitiveComponent.SetMaterial` (`self.StaticMesh`) 0 "/Game/Interactable_Objects/glow.glow")
  (bind _asbp_first_person_character (cast `/Game/FirstPerson/Blueprints/BP_FirstPersonCharacter` (stale `self.ReceiveActorEndOverlap` OtherActor)))
  (`Widget.SetVisibility` (`/Game/FirstPerson/Blueprints/BP_FirstPersonCharacter.e To Interact` _asbp_first_person_character) "Visible"))

(event `self.ReceiveActorEndOverlap`
  (params (OtherActor :type "Actor Object Reference"))
  (`PrimitiveComponent.SetMaterial` (`self.StaticMesh`) 0 (`self.originalMaterial`))
  (bind _asbp_first_person_character (cast `/Game/FirstPerson/Blueprints/BP_FirstPersonCharacter` OtherActor))
  (`Widget.SetVisibility` (`/Game/FirstPerson/Blueprints/BP_FirstPersonCharacter.e To Interact` _asbp_first_person_character) "Hidden"))

(fn `UserConstructionScript`)